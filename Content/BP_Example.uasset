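; Example actor that exercises a KK JSON parsing Blueprint library, printing the results.
; BeginPlay enables input, and pressing T parses the TestJsonObj and TestJsonArray strings in turn.
; Chained getters pass the JSON object along to read string, float, int, bool, nested object and array values, including an error-index check and a nested array.
; A LOG_VALUE helper prints each label with its value.
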(event EventBeginPlay
  (Input|EnableInput (Game|GetPlayerController 0)))

(event Input|KeyboardEvents|T
  (params (Key :type Key%20Structure :default "None"))
  (bind _test_json_obj (Variables|Default|Gettest_json_obj))
  (bind _test_json_array (Variables|Default|Gettest_json_array))
  (bind (_kkjsonvaluearray _returnvalue) (Class|KKJsonBlueprintFunctionLibrary|KKGetJsonArrayfromString _test_json_array))
  (bind (_kkjsonobject _returnvalue_2) (Class|KKJsonBlueprintFunctionLibrary|KKGetJsonObjectfromString _test_json_obj))
  (bind _kkjsonvalue (Class|KKJsonBlueprintFunctionLibrary|KKGetArrayValue _kkjsonvaluearray 2))
  (bind (_value _returnvalue_3) (Class|KKJsonBlueprintFunctionLibrary|KKGetValueString _kkjsonobject "strValue"))
  (bind _returnvalue_4 (Class|KKJsonBlueprintFunctionLibrary|KKasArray _kkjsonvalue))
  (bind (_value_2 _returnvalue_5) (Class|KKJsonBlueprintFunctionLibrary|KKGetValueFloat _returnvalue_3 "floatValue"))
  (bind (_value_3 _returnvalue_6) (Class|KKJsonBlueprintFunctionLibrary|KKGetValueInt _returnvalue_5 "intValue"))
  (bind (_value_4 _returnvalue_7) (Class|KKJsonBlueprintFunctionLibrary|KKGetValueBool _returnvalue_6 "boolValue"))
  (bind _returnvalue_8 (Class|KKJsonBlueprintFunctionLibrary|KKGetValueArray _returnvalue_7 "arrayValue"))
  (:Pressed
    (Utilities|FlowControl|Sequence
      (:then_0
        (if _returnvalue_2
          (Development|PrintString "get json obj success")
          (Utilities|LOGVALUE "get str value : " _value)
          (Utilities|LOGVALUE "get float value : " (Utilities|String|ToString(Float) _value_2))
          (Utilities|LOGVALUE "get int value : " (Utilities|String|ToString(Integer) _value_3))
          (Utilities|LOGVALUE "get int value : " (Utilities|String|ToString(Boolean) _value_4))
          (Utilities|LOGVALUE "get obj's string value : " (.Value (Class|KKJsonBlueprintFunctionLibrary|KKGetValueString (Class|KKJsonBlueprintFunctionLibrary|KKGetValueObject _returnvalue_7 "objValue") "objString")))
          (Utilities|FlowControl|Sequence
            (:then_0
              (Utilities|LOGVALUE "get array0's string value : " (Class|KKJsonBlueprintFunctionLibrary|KKasString (.KKJsonValue (Class|KKJsonBlueprintFunctionLibrary|KKGetArrayValue _returnvalue_8)))))
            (:then_1
              (Utilities|LOGVALUE "get array1's int value : " (Utilities|String|ToString(Integer) (Class|KKJsonBlueprintFunctionLibrary|KKasInt (.KKJsonValue (Class|KKJsonBlueprintFunctionLibrary|KKGetArrayValue _returnvalue_8 1))))))
            (:then_2
              (Utilities|LOGVALUE "get array error index : " (Utilities|String|ToString(Boolean) (.ReturnValue (Class|KKJsonBlueprintFunctionLibrary|KKGetArrayValue _returnvalue_8 2))))))))
      (:then_1
        (Development|PrintString "--------------------------------")
        (if _returnvalue
          (Development|PrintString "get json array success")
          (Utilities|FlowControl|Sequence
            (:then_0
              (Utilities|LOGVALUE "get array 0 : " (Class|KKJsonBlueprintFunctionLibrary|KKasString (.KKJsonValue (Class|KKJsonBlueprintFunctionLibrary|KKGetArrayValue _kkjsonvaluearray)))))
            (:then_1
              (Utilities|LOGVALUE "get array 1: " (Class|KKJsonBlueprintFunctionLibrary|KKasString (.KKJsonValue (Class|KKJsonBlueprintFunctionLibrary|KKGetArrayValue _kkjsonvaluearray 1)))))
            (:then_2
              (Utilities|LOGVALUE "get array 2's array 0 : " (Class|KKJsonBlueprintFunctionLibrary|KKasString (.KKJsonValue (Class|KKJsonBlueprintFunctionLibrary|KKGetArrayValue _returnvalue_4))))
              (Utilities|LOGVALUE "get array 2's array 1 : " (Class|KKJsonBlueprintFunctionLibrary|KKasString (.KKJsonValue (Class|KKJsonBlueprintFunctionLibrary|KKGetArrayValue _returnvalue_4 1)))))
            (:then_3
              (Utilities|LOGVALUE "get array 3 : " (Class|KKJsonBlueprintFunctionLibrary|KKasString (.KKJsonValue (Class|KKJsonBlueprintFunctionLibrary|KKGetArrayValue _kkjsonvaluearray 3)))))))))))

(fn ConstructionScript)